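; BP_Door is a hub door that swings open when the third-person character is inside its Trigger and closes when none remains.
; Tick polls the trigger's overlaps and uses IsOpen and IsMoving to start the OpenDoor or CloseDoor timeline.
; Each timeline drives the Door's relative yaw from its DoorAngle track, setting IsOpen and clearing IsMoving on every update rather than on finish.
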(event `self.ReceiveTick`
  (params (DeltaSeconds :type "Float (single-precision)"))
  (bind _door (`self.Door`))
  (if (`self.IsMoving`)
    _
    (elif (> (`KismetArrayLibrary.Array_Length` (`PrimitiveComponent.GetOverlappingActors` (`self.Trigger`) "/Game/ThirdPerson/Blueprints/BP_ThirdPersonCharacter.BP_ThirdPersonCharacter_C")) 0)
      (if (not (`self.IsOpen`))
        (set `self.IsMoving` true)
        (bind (_direction _doorangle) (`Timeline|OpenDoor` :!via `PlayFromStart`)
          (:`Update`
            (`SceneComponent.K2_SetRelativeRotation` _door (`KismetMathLibrary.MakeRotator` 0.0 0.0 _doorangle) false false)
            (set `self.IsOpen` true)
            (set `self.IsMoving` false))))
      (elif (`self.IsOpen`)
        (set `self.IsMoving` true)
        (bind (_direction_2 _doorangle_2) (`Timeline|CloseDoor` :!via `PlayFromStart`)
          (:`Update`
            (`SceneComponent.K2_SetRelativeRotation` _door (`KismetMathLibrary.MakeRotator` 0.0 0.0 _doorangle_2) false false)
            (set `self.IsOpen` false)
            (set `self.IsMoving` false)))))))

(fn `UserConstructionScript`)