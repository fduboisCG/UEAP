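; BP_IceZone is a trigger zone that makes a player's snowboard rotate more loosely while inside it.
; On overlap begin, it casts the actor to BP_ThirdPersonCharacter and its CurrVehicle to BP_Snowboard, then subtracts DamplingDecrease from the board's AngularDampingForce.
; On overlap end, it repeats the lookup and adds the same amount back, relying on symmetric offsets rather than a stored original value.
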(event `self.IceZone.OnComponentBeginOverlap`
  (params (OverlappedComponent :type "PrimitiveComponent Object Reference") (OtherActor :type "Actor Object Reference") (OtherComp :type "PrimitiveComponent Object Reference") (OtherBodyIndex :type Integer) (bFromSweep :type Boolean) (SweepResult :type "HitResult Structure (by ref)"))
  (bind _asbp_third_person_character (cast `/Game/ThirdPerson/Blueprints/BP_ThirdPersonCharacter` OtherActor))
  (bind _asbp_snowboard (cast `/Game/01-Blueprints/Snowboard/BP_Snowboard` (`/Game/ThirdPerson/Blueprints/BP_ThirdPersonCharacter.Curr_Vehicle` _asbp_third_person_character)))
  (set `/Game/01-Blueprints/Snowboard/BP_Snowboard.Angular_Damping_Force` (- (`/Game/01-Blueprints/Snowboard/BP_Snowboard.Angular_Damping_Force` _asbp_snowboard) (`self.DamplingDecrease`)) _asbp_snowboard))

(event `self.IceZone.OnComponentEndOverlap`
  (params (OverlappedComponent :type "PrimitiveComponent Object Reference") (OtherActor :type "Actor Object Reference") (OtherComp :type "PrimitiveComponent Object Reference") (OtherBodyIndex :type Integer))
  (bind _asbp_third_person_character (cast `/Game/ThirdPerson/Blueprints/BP_ThirdPersonCharacter` OtherActor))
  (bind _asbp_snowboard (cast `/Game/01-Blueprints/Snowboard/BP_Snowboard` (`/Game/ThirdPerson/Blueprints/BP_ThirdPersonCharacter.Curr_Vehicle` _asbp_third_person_character)))
  (set `/Game/01-Blueprints/Snowboard/BP_Snowboard.Angular_Damping_Force` (+ (`/Game/01-Blueprints/Snowboard/BP_Snowboard.Angular_Damping_Force` _asbp_snowboard) (`self.DamplingDecrease`)) _asbp_snowboard))

(fn `UserConstructionScript`)