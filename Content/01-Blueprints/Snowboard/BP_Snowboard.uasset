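; Rideable physics snowboard pawn that the player character attaches to and possesses, then detaches from on exit.
; Four downward traces apply distance-scaled hover force, with mass-based drive forces and torque steering from IA_Move.
; Tick adds damping, rotation limits, a speed cap and constant wind impulse.
; A ground trace weakens forward thrust and damping in air and gates the Niagara snow trail, while forward speed widens camera FOV.
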(event `Initialize_Forces`
  (`self.Calculate_Hover_Force`)
  (`self.Calculate_Movement_Force`))

(event `self.ReceiveBeginPlay`
  (`self.Initialize_Hover`))

(event `self.ReceiveTick`
  (params (DeltaSeconds :type "Float (single-precision)"))
  (bind _maxvelocity (`self.MaxVelocity`))
  (`self.Get_Grounded`)
  (`self.Apply_Hover_Force`)
  (`self.Apply_Linear_Dampling`)
  (`self.Apply_Angular_Dampling`)
  (`self.Limit_Rotation`)
  (`self.Display_Niagara`)
  (`self.ChangeFOV`)
  (`self.Apply_Wind`)
  (bind _returnvalue (`PrimitiveComponent.GetPhysicsLinearVelocity` (`self.SM_Snowboard`) "None"))
  (bind _returnvalue_2 (`KismetMathLibrary.VSize` _returnvalue))
  (if (>= _returnvalue_2 _maxvelocity)
    (`PrimitiveComponent.SetPhysicsLinearVelocity` (`self.SM_Snowboard`) (/ (* _returnvalue _maxvelocity) _returnvalue_2) false "None")))

(event `EnhancedInput|/Game/03-Inputs/Actions/IA_Move`
  (params (ActionValue :type "Vector2D Structure") (ElapsedSeconds :type "Float (double-precision)") (TriggeredSeconds :type "Float (double-precision)") (InputAction :type "InputAction Object Reference" :default "/Game/03-Inputs/Actions/IA_Move.IA_Move"))
  (:`Triggered`
    (`self.Apply_Movement` ActionValue)))

(event `/Game/01-Blueprints/Interfaces/BPI_Vehicle.Enter_Vehicle`
  ;[1 1 1] Enter Vehicle
  (bind _output_get (set `self.Curr_Driver` (`GameplayStatics.GetPlayerCharacter` 0)))
  (`self.Initialize_Forces`)
  (`self.K2_AttachToActor` _output_get self "Character_Seat" "SnapToTarget" "SnapToTarget" "KeepWorld" true)
  (`Controller.Possess` (`GameplayStatics.GetPlayerController` 0) self)
  (`CharacterMovementComponent.SetMovementMode` (`Character.CharacterMovement` (`self.Curr_Driver`)) "MOVE_Flying" 0)
  (set `self.Turn_On` true))

(event `ExitVehicle`
  (bind _curr_driver (`self.Curr_Driver`))
  ;[1 1 1] Exit Vehicle
  (bind _curr_driver_2 (`self.Curr_Driver`)
    (:`then`
      (`self.K2_DetachFromActor` _curr_driver_2 "KeepWorld" "KeepWorld" "KeepWorld")
      (`self.K2_SetActorLocation` _curr_driver_2 (`SceneComponent.K2_GetComponentLocation` (`self.Exit_Location`)) false false)
      (`Controller.Possess` (`GameplayStatics.GetPlayerController` 0) _curr_driver)
      (`CharacterMovementComponent.SetMovementMode` (`Character.CharacterMovement` _curr_driver) "MOVE_Walking" 0)
      (set `self.Curr_Driver` null)
      (set `self.Turn_On` false))
    (:`else`)))

(fn `Apply_Angular_Dampling`
  (bind _sm_snowboard (`self.SM_Snowboard`))
  (if (`self.Turn_On`)
    (`PrimitiveComponent.AddTorqueInRadians` (`self.SM_Snowboard`) (* (* (`PrimitiveComponent.GetPhysicsAngularVelocityInRadians` _sm_snowboard "None") -1.0) (* (`PrimitiveComponent.GetInertiaTensor` _sm_snowboard "None") (`self.Angular_Damping_Force`))) "None" false)))

(fn `Apply_Hover_Force`
  (if (`self.Turn_On`)
    (for _array_element (`self.HoverPoints`)
      (bind _returnvalue (`SceneComponent.K2_GetComponentLocation` _array_element))
      (bind (_outhit _returnvalue_2) (`KismetSystemLibrary.LineTraceSingle` :`Start` _returnvalue :`End` (+ _returnvalue (* (`KismetMathLibrary.MakeVector` 0.0 0.0 -1.0) (`self.Hover_Distance`))) :`TraceChannel` "TraceTypeQuery1" :`DrawDebugType` "ForDuration" :`DrawTime` 0.0))
      (if _returnvalue_2
        (`PrimitiveComponent.AddForceAtLocation` (`self.SM_Snowboard`) (* (`SceneComponent.GetUpVector` (`self.SM_Snowboard`)) (/ (`self.Hover_Force`) (`.Distance` (`GameplayStatics.BreakHitResult` _outhit)))) (`SceneComponent.K2_GetComponentLocation` _array_element) "None")))))

(fn `Apply_Linear_Dampling`
  (bind _linear_damping_force (`self.Linear_Damping_Force`))
  (`PrimitiveComponent.AddForce` (`self.SM_Snowboard`) (* (* (`SceneComponent.GetComponentVelocity` (`self.SM_Snowboard`)) -1.0) (`KismetMathLibrary.SelectFloat` _linear_damping_force (/ _linear_damping_force 4.0) (`self.Is_Grounded?`))) "None" false))

(fn `Apply_Movement`
  (params (Move_Input :type "Vector2D Structure"))
  (bind _forward_force (`self.Forward_Force`))
  (`PrimitiveComponent.AddTorqueInRadians` (`self.SM_Snowboard`) (* (* (`SceneComponent.GetUpVector` (`self.SM_Snowboard`)) (`self.Turn_Force`)) Move_Input_X) "None" false)
  (if (> Move_Input_Y 0.0)
    (`PrimitiveComponent.AddForce` (`self.SM_Snowboard`) (* (`SceneComponent.GetForwardVector` (`self.SM_Snowboard`)) (`KismetMathLibrary.SelectFloat` _forward_force (/ _forward_force 5.0) (`self.Is_Grounded?`))) "None" false)
    (else
      (`PrimitiveComponent.AddForce` (`self.SM_Snowboard`) (* (* (`SceneComponent.GetForwardVector` (`self.SM_Snowboard`)) -1.0) (`self.Backward_Force`)) "None" false))))

(fn `Apply_Wind`
  (`PrimitiveComponent.AddImpulse` (`self.SM_Snowboard`) (* (`self.WindForce`) (`KismetMathLibrary.Normal` (`self.WindDirection`))) "None" true))

(fn `Calculate_Hover_Force`
  (set `self.Hover_Force` (* (* (+ (`PrimitiveComponent.GetMass` (`self.SM_Snowboard`)) (`CharacterMovementComponent.Mass` (`Character.CharacterMovement` (`self.Curr_Driver`)))) (`self.Hover_Acceleration`)) 100.0)))

(fn `Calculate_Movement_Force`
  (bind _returnvalue (+ (`PrimitiveComponent.GetMass` (`self.SM_Snowboard`)) (`CharacterMovementComponent.Mass` (`Character.CharacterMovement` (`self.Curr_Driver`)))))
  (set `self.Forward_Force` (* (* _returnvalue (`self.Forward_Acceleration`)) 100.0))
  (set `self.Backward_Force` (* (* _returnvalue (`self.Backward_Acceleration`)) 100.0))
  (set `self.Turn_Force` (`KismetMathLibrary.VSize` (* (`PrimitiveComponent.GetInertiaTensor` (`self.SM_Snowboard`) "None") (`self.Turn_Acceleration`)))))

(fn `ChangeFOV`
  (bind _sm_snowboard (`self.SM_Snowboard`))
  (bind _camera (`self.Camera`))
  (bind _returnvalue (`PrimitiveComponent.GetPhysicsLinearVelocity` _sm_snowboard "None"))
  (`CameraComponent.SetFieldOfView` _camera (`KismetMathLibrary.FInterpTo` (`CameraComponent.FieldOfView` _camera) (`KismetMathLibrary.MapRangeClamped` (`KismetMathLibrary.Dot_VectorVector` _returnvalue (`SceneComponent.GetForwardVector` _sm_snowboard)) 0.0 1000.0 90.0 (`self.MaxFOV`)) (`GameplayStatics.GetWorldDeltaSeconds`) 5.0)))

(fn `Display_Niagara`
  (bind _snowtrail (`self.SnowTrail`))
  (if (`self.IsOnSnow`)
    (if (`self.Is_Grounded?`)
      (bind _returnvalue (`PrimitiveComponent.GetPhysicsLinearVelocity` (`self.SM_Snowboard`) "None"))
      (bind _returnvalue_x (`KismetMathLibrary.BreakVector` (* _returnvalue (`SceneComponent.GetForwardVector` (`self.SM_Snowboard`)))))
      (if (>= _returnvalue_x 10.0)
        (bind _returnvalue_2 (`NiagaraFunctionLibrary.SpawnSystemAtLocation` "/Game/06-Niagara/NS_SnowTrail.NS_SnowTrail" (`SceneComponent.K2_GetComponentLocation` _snowtrail) (`SceneComponent.K2_GetComponentRotation` _snowtrail)))
        (`NiagaraComponent.SetNiagaraVariableFloat` _returnvalue_2 "SpawnRate" _returnvalue_x)))))

(fn `Get_Grounded`
  (bind _returnvalue (`SceneComponent.K2_GetComponentLocation` (`self.SM_Snowboard`)))
  (bind (_outhit _returnvalue_2) (`KismetSystemLibrary.LineTraceSingle` :`Start` _returnvalue :`End` (+ _returnvalue (* (`KismetMathLibrary.MakeVector` 0.0 0.0 -1.0) (`self.Check_Ground_Distance`))) :`TraceChannel` "TraceTypeQuery1" :`DrawDebugType` "ForDuration" :`TraceColor` (struct :`G` 0.759831 :`B` 1.0 :`A` 1.0) :`DrawTime` 0.0))
  (set `self.Is_Grounded?` _returnvalue_2))

(fn `Initialize_Hover`
  (set `self.HoverPoints` (`|MakeArray` (`self.Hover_Point_1`) (`self.Hover_Point_2`) (`self.Hover_Point_3`) (`self.Hover_Point_4`) :!type "SceneComponent Object Reference")))

(fn `Limit_Rotation`
  (bind (_returnvalue_roll _returnvalue_pitch _returnvalue_yaw) (`KismetMathLibrary.BreakRotator` (`SceneComponent.K2_GetComponentRotation` (`self.SM_Snowboard`))))
  (if (`self.Turn_On`)
    (`SceneComponent.K2_SetWorldRotation` (`self.SM_Snowboard`) (`KismetMathLibrary.MakeRotator` (`KismetMathLibrary.FClamp` _returnvalue_roll (/ (`self.Min_Rotation_Angle`) 2.0) (/ (`self.Max_Rotation_Angle`) 2.0)) (`KismetMathLibrary.FClamp` _returnvalue_pitch (`self.Min_Rotation_Angle`) (`self.Max_Rotation_Angle`)) _returnvalue_yaw) false false)))

(fn `UserConstructionScript`)