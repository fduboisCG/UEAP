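; BP_SnowballSpawner is an actor that repeatedly spawns snowballs at its own location.
; On BeginPlay it starts a looping timer that calls SpawnSnowball at the configured spawn interval.
; Each spawned BP_Snowball receives the spawner's waypoints, speed and rotation speed, so each spawner instance defines the path and motion of its snowballs.
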(event `self.ReceiveBeginPlay`
  (`KismetSystemLibrary.K2_SetTimer` null "SpawnSnowball" (`self.SnowballSpawnTime`) true))

(event `SpawnSnowball`
  (bind _returnvalue (`|SpawnActorFromClass` (`self.SnowballClass`) (`KismetMathLibrary.MakeTransform` (`SceneComponent.K2_GetComponentLocation` (`self.DefaultSceneRoot`))) "Undefined" "MultiplyWithRoot" null null))
  (bind _asbp_snowball (cast `/Game/01-Blueprints/Snowball/BP_Snowball` _returnvalue))
  (set `/Game/01-Blueprints/Snowball/BP_Snowball.Waypoints` (`self.Waypoints`) _asbp_snowball)
  (set `/Game/01-Blueprints/Snowball/BP_Snowball.Speed` (`self.SnowballSpeed`) _asbp_snowball)
  (set `/Game/01-Blueprints/Snowball/BP_Snowball.RotationSpeed` (`self.SnowballRotation`) _asbp_snowball))

(fn `UserConstructionScript`)