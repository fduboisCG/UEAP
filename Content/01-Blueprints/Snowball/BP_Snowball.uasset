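; BP_Snowball is a rolling snowball actor that follows a waypoint path and shatters when something overlaps its interaction area.
; Tick moves the geometry collection at constant speed with sweep, adds roll, and destroys the actor after the last waypoint.
; On overlap it enables physics, fires a short-lived BP_SnowballMasterField to break the collection, then destroys itself after DestroyTime.
; BeginPlay stores a dynamic snow material instance.
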(event `self.ReceiveBeginPlay`
  (bind _returnvalue (`PrimitiveComponent.CreateDynamicMaterialInstance` (`self.GeometryCollection`) 0 "/Game/04-Materials/M_Snow.M_Snow" "None"))
  (set `self.MaterialInstance` _returnvalue))

(event `self.InteractionArea.OnComponentBeginOverlap`
  (params (OverlappedComponent :type "PrimitiveComponent Object Reference") (OtherActor :type "Actor Object Reference") (OtherComp :type "PrimitiveComponent Object Reference") (OtherBodyIndex :type Integer) (bFromSweep :type Boolean) (SweepResult :type "HitResult Structure (by ref)"))
  (`PrimitiveComponent.SetSimulatePhysics` (`self.GeometryCollection`) true)
  (`self.DestroySnowball`)
  (`KismetSystemLibrary.Delay` (`self.DestroyTime`))
  (`self.K2_DestroyActor`))

(event `self.ReceiveTick`
  (params (DeltaSeconds :type "Float (single-precision)"))
  (bind (_returnvalue_roll _returnvalue_pitch _returnvalue_yaw) (`KismetMathLibrary.BreakRotator` (`SceneComponent.K2_GetComponentRotation` (`self.GeometryCollection`))))
  (bind _returnvalue (`self.K2_GetActorLocation` (`|GetArrayItem` (`self.Waypoints`) (`self.CurrentWaypointIndex`))))
  (if (< (`self.CurrentWaypointIndex`) (`KismetArrayLibrary.Array_Length` (`self.Waypoints`)))
    (`SceneComponent.K2_SetWorldLocation` (`self.GeometryCollection`) (`KismetMathLibrary.VInterpTo_Constant` (`SceneComponent.K2_GetComponentLocation` (`self.GeometryCollection`)) _returnvalue DeltaSeconds (`self.Speed`)) true false)
    (`SceneComponent.K2_SetWorldRotation` (`self.GeometryCollection`) (`KismetMathLibrary.MakeRotator` (+ _returnvalue_roll (* (`self.RotationSpeed`) DeltaSeconds)) _returnvalue_pitch _returnvalue_yaw) false false)
    (if (< (`KismetMathLibrary.Vector_Distance` (`SceneComponent.K2_GetComponentLocation` (`self.GeometryCollection`)) _returnvalue) DeltaSeconds)
      (`/Engine/EditorBlueprintResources/StandardMacros.IncrementInt` (`self.CurrentWaypointIndex`)
        (:`  `
          (if (== (`self.CurrentWaypointIndex`) (`KismetArrayLibrary.Array_Length` (`self.Waypoints`)))
            (`self.K2_DestroyActor`)))))))

(fn `DestroySnowball`
  (bind _returnvalue (`|SpawnActorFromClass` "/Game/01-Blueprints/Snowball/BP_SnowballMasterField.BP_SnowballMasterField_C" (`KismetMathLibrary.MakeTransform` (`SceneComponent.K2_GetComponentLocation` (`self.GeometryCollection`)) (struct) (10.0 10.0 10.0)) "AlwaysSpawn" "MultiplyWithRoot" null null))
  (set `/Engine/EditorResources/FieldNodes/FS_MasterField.ActivationType` "NewEnumerator4" _returnvalue)
  (`/Engine/EditorResources/FieldNodes/FS_MasterField.CE_Trigger` _returnvalue)
  (`self.K2_DestroyActor` _returnvalue))

(fn `UserConstructionScript`)