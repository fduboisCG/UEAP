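; BP_WindZone is a trigger volume that applies wind to the snowboard the player character is riding.
; On overlap begin, it casts the character's current vehicle to BP_Snowboard and writes the zone's WindForce and the Arrow component's forward vector as the wind direction.
; On overlap end, it resets both values to zero, leaving any use of the wind to the snowboard.
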(event `self.WindZone.OnComponentBeginOverlap`
  (params (OverlappedComponent :type "PrimitiveComponent Object Reference") (OtherActor :type "Actor Object Reference") (OtherComp :type "PrimitiveComponent Object Reference") (OtherBodyIndex :type Integer) (bFromSweep :type Boolean) (SweepResult :type "HitResult Structure (by ref)"))
  (bind _asbp_third_person_character (cast `/Game/ThirdPerson/Blueprints/BP_ThirdPersonCharacter` OtherActor))
  (bind _asbp_snowboard (cast `/Game/01-Blueprints/Snowboard/BP_Snowboard` (`/Game/ThirdPerson/Blueprints/BP_ThirdPersonCharacter.Curr_Vehicle` _asbp_third_person_character)))
  (set `/Game/01-Blueprints/Snowboard/BP_Snowboard.WindForce` (`self.WindForce`) _asbp_snowboard)
  (set `/Game/01-Blueprints/Snowboard/BP_Snowboard.WindDirection` (`SceneComponent.GetForwardVector` (`self.Arrow`)) _asbp_snowboard))

(event `self.WindZone.OnComponentEndOverlap`
  (params (OverlappedComponent :type "PrimitiveComponent Object Reference") (OtherActor :type "Actor Object Reference") (OtherComp :type "PrimitiveComponent Object Reference") (OtherBodyIndex :type Integer))
  (bind _asbp_third_person_character (cast `/Game/ThirdPerson/Blueprints/BP_ThirdPersonCharacter` OtherActor))
  (bind _asbp_snowboard (cast `/Game/01-Blueprints/Snowboard/BP_Snowboard` (`/Game/ThirdPerson/Blueprints/BP_ThirdPersonCharacter.Curr_Vehicle` _asbp_third_person_character)))
  (set `/Game/01-Blueprints/Snowboard/BP_Snowboard.WindForce` 0.0 _asbp_snowboard)
  (set `/Game/01-Blueprints/Snowboard/BP_Snowboard.WindDirection` (0.0 0.0 0.0) _asbp_snowboard))

(fn `UserConstructionScript`)