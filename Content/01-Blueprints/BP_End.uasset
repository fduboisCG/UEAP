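; BP_End is a finish trigger that ends a snowboard run with a win.
; When a third-person character riding a BP_Snowboard overlaps the trigger box, it waits briefly, makes the board eject the rider, then calls Win on the character.
; DisplayWin spawns a Niagara confetti burst at the Confetti component's location and rotation.
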(event `self.TriggerBox.OnComponentBeginOverlap`
  (params (OverlappedComponent :type "PrimitiveComponent Object Reference") (OtherActor :type "Actor Object Reference") (OtherComp :type "PrimitiveComponent Object Reference") (OtherBodyIndex :type Integer) (bFromSweep :type Boolean) (SweepResult :type "HitResult Structure (by ref)"))
  (bind _asbp_third_person_character (cast `/Game/ThirdPerson/Blueprints/BP_ThirdPersonCharacter` OtherActor))
  (bind _asbp_snowboard (cast `/Game/01-Blueprints/Snowboard/BP_Snowboard` (`/Game/ThirdPerson/Blueprints/BP_ThirdPersonCharacter.Curr_Vehicle` _asbp_third_person_character)))
  (`KismetSystemLibrary.Delay` 1.0)
  (`/Game/01-Blueprints/Snowboard/BP_Snowboard.ExitVehicle` _asbp_snowboard)
  (`self.DisplayWin`)
  (`/Game/ThirdPerson/Blueprints/BP_ThirdPersonCharacter.Win` _asbp_third_person_character))

(fn `DisplayWin`
  (bind _confetti (`self.confetti`))
  (`NiagaraFunctionLibrary.SpawnSystemAtLocation` "/Game/06-Niagara/NS_Confetti.NS_Confetti" (`SceneComponent.K2_GetComponentLocation` _confetti) (`SceneComponent.K2_GetComponentRotation` _confetti)))

(fn `UserConstructionScript`)